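; BP_NPC is an AI character meant to chase BP_FirstPersonCharacter on sight and wander otherwise, though neither chain is wired to an event, so neither runs.
; The sight chain sets CanSeeEnemy and moves to the player, with a 0.5-second retriggerable delay clearing the flag when sightings stop.
; The chain labeled as Tick waits a random interval while the flag is false, then moves to a random reachable nearby point.
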(fn ConstructionScript)