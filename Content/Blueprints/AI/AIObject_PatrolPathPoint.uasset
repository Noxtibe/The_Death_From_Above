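; AI patrol path point actor that turns an arriving patroller to face the direction of the point's arrow.
; When a patroller enters, it stores the character, opens a gate and fires a point-met call.
; While the gate is open, Tick smoothly interpolates the character's rotation toward the arrow's world rotation at the rotation speed.
; The exit event closes the gate to stop the turning.
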(event Custom|On%20Patroller%20Entered
  (params (Character :type Character%20Object%20Reference))
  (Variables|Default|SetCharacter Character)
  (Utilities|FlowControl|Sequence
    (:then_0
      (Utilities|FlowControl|Gate true) ; enters at Open
    )
    (:then_1
      (Default|CallOnPointMet))))

(event Custom|On%20Patroller%20Exit
  (bind _character (Variables|Default|GetCharacter))
  (Utilities|FlowControl|Gate true) ; enters at Close
)

(event EventTick
  (params (DeltaSeconds :type Float%20%28single-precision%29))
  (bind _character (Variables|Default|GetCharacter))
  (Utilities|FlowControl|Gate true
    (:Exit
      (Utilities|IsValid _character
        (:Is%20Valid
          (Transformation|SetActorRotation _character (Math|Interpolation|RInterpTo (Transformation|GetActorRotation (Variables|Default|GetCharacter)) (Transformation|GetWorldRotation (Variables|Default|GetArrow)) DeltaSeconds (Variables|Default|GetRotation%20Speed))))))))

(fn ConstructionScript)