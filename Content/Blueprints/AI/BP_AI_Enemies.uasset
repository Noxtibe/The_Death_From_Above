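; BP_AI_Enemies is an enemy AI character that the player can take down.
; Overlapping TakedownArea toggles CanTakedown on BP_Player.
; The Takedown event disables movement and collision, plays a death-from-the-back animation, then destroys the actor after a delay.
; Hits report touch events to AI perception, while the sight-chase and random-patrol logic is present but disconnected, with an unresolved cast.
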(event OnComponentBeginOverlap(TakedownArea)
  (params (OverlappedComponent :type Primitive%20Component%20Object%20Reference) (OtherActor :type Actor%20Object%20Reference) (OtherComp :type Primitive%20Component%20Object%20Reference) (OtherBodyIndex :type Integer) (bFromSweep :type Boolean) (SweepResult :type Hit%20Result%20Structure%20%28by%20ref%29))
  (bind _asbp_player (Utilities|Casting|CastToBP_Player OtherActor))
  (Variables|/Game/Blueprints/Player/BP_Player.BP_Player_C|SetCan%20Takedown _asbp_player true))

(event OnComponentEndOverlap(TakedownArea)
  (params (OverlappedComponent :type Primitive%20Component%20Object%20Reference) (OtherActor :type Actor%20Object%20Reference) (OtherComp :type Primitive%20Component%20Object%20Reference) (OtherBodyIndex :type Integer))
  (bind _asbp_player (Utilities|Casting|CastToBP_Player OtherActor))
  (Variables|/Game/Blueprints/Player/BP_Player.BP_Player_C|SetCan%20Takedown _asbp_player false))

(event Custom|Takedown
  (Pawn|Components|CharacterMovement|DisableMovement (Variables|Character|GetCharacterMovement))
  (Collision|SetActorEnableCollision false)
  (Components|Animation|PlayAnimation (Variables|Character|GetMesh) "/Game/Animations/Anim_Death_From_The_Back.Anim_Death_From_The_Back" false)
  (Utilities|FlowControl|Delay 1e+01)
  (Actor|DestroyActor))

(event Collision|EventHit
  (params (MyComp :type Primitive%20Component%20Object%20Reference) (Other :type Actor%20Object%20Reference) (OtherComp :type Primitive%20Component%20Object%20Reference) (bSelfMoved :type Boolean) (HitLocation :type Vector :default "0, 0, 0") (HitNormal :type Vector :default "0, 0, 0") (NormalImpulse :type Vector :default "0, 0, 0") (Hit :type Hit%20Result%20Structure%20%28by%20ref%29))
  (Class|AISenseTouch|ReportTouchEvent self Other HitLocation))

(fn ConstructionScript)