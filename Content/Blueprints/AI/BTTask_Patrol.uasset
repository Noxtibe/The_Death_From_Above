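; Behavior tree task that walks an AI pawn along the patrol path stored in its AC_AIBehavior component.
; The path maps point actors to wait times; the pawn moves to each, notifies it on entry and exit, and waits on a timer.
; At either end it loops or reverses per PatrolPathOutcome, repeating the endpoint when reversing.
; The task only finishes, as failed, on missing component, empty path or failed move.
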(event Custom|MoveToPatrolPoint
  (bind _patrol_path (Variables|Default|GetPatrol%20Path))
  ;[0 0.8794 1] Path for the AI to follow with pause
  ;;[1 1 1] Get all keys in the map
  (bind _keys (Utilities|Map|Keys (Variables|Default|GetPatrol%20Path)))
  (AI|AIMoveTo (Variables|Default|GetControlled%20Pawn) (Transformation|GetActorLocation (Utilities|Array|Get(acopy) _keys (Variables|Default|GetCurrent%20Patrol%20Index))) 0 5.0 false
    (:OnSuccess
      (bind _keys_2 (Utilities|Map|Keys _patrol_path))
      (Variables|Default|SetCurrent%20Patrol%20Point (Utilities|Array|Get(acopy) _keys_2 (Variables|Default|GetCurrent%20Patrol%20Index)))
      ;;[1 1 1] AI Waiting to move with given time
      (Utilities|Time|SetTimerbyEvent (delegate Custom|OnEndWaiting) (Math|Float|Max(Float) (.Value (Utilities|Map|Find _patrol_path (Utilities|Array|Get(acopy) _keys_2 (Variables|Default|GetCurrent%20Patrol%20Index)))) 0.1))
      (Default|OnPatrollerEntered (Variables|Default|GetCurrent%20Patrol%20Point) (.AsCharacter (Utilities|Casting|CastToCharacter (Variables|Default|GetControlled%20Pawn)))))
    (:OnFail
      (AI|BehaviorTree|FinishExecute false))))

(event Custom|OnEndWaiting
  ;[0 0.8794 1] Path for the AI to follow with pause
  ;;[1 1 1] Incrémente l'index de +1 pour continuer la patrouille
  (Default|OnPatrollerExit (Variables|Default|GetCurrent%20Patrol%20Point))
  (bind _output_get (Variables|Default|SetCurrent%20Patrol%20Index (+ (Variables|Default|GetCurrent%20Patrol%20Index) (Variables|Default|GetPath%20Direction))))
  (if (CallFunction|IsValidMapIndex _output_get)
    (CallFunction|MovetoPatrolPoint)
    (else
      ;;[1 1 1] Choose behavior
      (switch Utilities|FlowControl|Switch|SwitchonEPatrolPathOutcome (Variables|Default|GetPatrol%20Path%20Outcome)
        (:NewEnumerator0
          ;;[1 1 1] Infinite loop on patrol path
          (Variables|Default|SetCurrent%20Patrol%20Index 0)
          (CallFunction|MovetoPatrolPoint))
        (:NewEnumerator1
          ;;[1 1 1] Reverse patrol
          (Variables|Default|SetPath%20Direction (* (Variables|Default|GetPath%20Direction) -1))
          (Variables|Default|SetCurrent%20Patrol%20Index (+ (Variables|Default|GetCurrent%20Patrol%20Index) (Variables|Default|GetPath%20Direction)))
          (CallFunction|MovetoPatrolPoint))))))

(event EventReceiveExecuteAI
  (params (OwnerController :type AI%20Controller%20Object%20Reference) (ControlledPawn :type Pawn%20Object%20Reference))
  (bind _returnvalue (Actor|GetComponentbyClass ControlledPawn "/Game/Blueprints/AI/AC_AIBehavior.AC_AIBehavior_C"))
  ;[0 0.04621 0.224] Vérirfication du component et du patrol path
  (Variables|Default|SetControlled%20Pawn ControlledPawn)
  ;;[1 1 1] Valid AI Component
  (Utilities|IsValid _returnvalue
    (:Is%20Valid
      (Variables|Default|SetPatrol%20Path%20Outcome (Variables|/Game/Blueprints/AI/AC_AIBehavior.AC_AIBehavior_C|GetPatrol%20Path%20Outcome _returnvalue))
      ;;[1 1 1] Patrol Path Assigned
      (if (> (Utilities|Map|Length (Variables|/Game/Blueprints/AI/AC_AIBehavior.AC_AIBehavior_C|GetPatrol%20Path _returnvalue)) 0)
        (Variables|Default|SetPatrol%20Path (Variables|/Game/Blueprints/AI/AC_AIBehavior.AC_AIBehavior_C|GetPatrol%20Path _returnvalue))
        (CallFunction|MovetoPatrolPoint)
        (else
          (AI|BehaviorTree|FinishExecute false))))
    (:Is%20Not%20Valid
      (AI|BehaviorTree|FinishExecute false))))

(fn IsValidMapIndex
  (params (IndexToTest :type Integer))
  (bind _keys (Utilities|Map|Keys (Variables|Default|GetPatrol%20Path)))
  (return (Utilities|Array|IsValidIndex _keys IndexToTest)))